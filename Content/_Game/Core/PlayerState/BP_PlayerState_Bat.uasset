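; Player state for the bat that tracks score, lives and the bat's current state during a level.
; On BeginPlay it restores lives and score from the persistent game instance and pushes them to the player controller through message calls.
; Score and lives events add to the running totals and notify the controller; life changes also message the pawn, or open TitleScreen when lives drop below zero.
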(event `self.ReceiveBeginPlay`
  ;[1 1 1] Update Level Score and Lives from Persistent Game Instance
  (bind (_lives _score) (message `I_Framework.RetrievePersistentData` (`GameplayStatics.GetGameInstance`)))
  (bind _output_get (set `self.PlayerLives` _lives))
  (message `I_Framework.LivesUpdate` (`self.GetPlayerController`) _output_get)
  (bind _output_get_2 (set `self.CurrentScore` _score))
  (message `I_Framework.ScoreUpdate` (`self.GetPlayerController`) _output_get_2))

(event `self.ScoreUpdate`
  (params (points :type Integer))
  ;[1 1 1] Update Score During Level
  (bind _output_get (set `self.CurrentScore` (+ points (`self.CurrentScore`))))
  (message `I_Framework.ScoreUpdate` (`GameplayStatics.GetPlayerController` 0) _output_get))

(event `self.LivesUpdate`
  (params (lives :type Integer))
  ;[1 1 1] Update Lives During Level
  (bind _output_get (set `self.PlayerLives` (+ lives (`self.PlayerLives`))))
  (if (< _output_get 0)
    (`GameplayStatics.OpenLevel` "TitleScreen")
    (else
      (message `I_Framework.LivesUpdate` (`GameplayStatics.GetPlayerPawn` 0) 0)
      (message `I_Framework.LivesUpdate` (`GameplayStatics.GetPlayerController` 0) _output_get))))

(fn `Change Player State`
  (params (`New State` :type "/Game/_Game/Core/PlayerState/ENUM_BatState Enum" :default "NewEnumerator0"))
  (if (`|EnumInequality` `New State` (`self.Bat State`))
    (set `self.Bat State` `New State`)))

(fn `RetrievePersistentData`
  (returns (lives :type Integer) (score :type Integer))
  (return 0 0))

(fn `UserConstructionScript`)