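; Player controller for a bat-and-ball game that drives the possessed BP_Bat and shows the score.
; On possess it stores the bat, has it spawn a ball and adds a WBP_Score widget to the viewport, which ScoreUpdate refreshes with points.
; The Move axis, scaled by mouse sensitivity, picks the bat's left, right or stop call and feeds its timeline play rate to set movement speed.
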(event `self.ScoreUpdate`
  (params (points :type Integer))
  (`/Game/_Game/UI/WBP_Score.Update Score` (`self.Displayed Score`) points))

(event `self.ReceivePossess`
  (params (PossessedPawn :type "Pawn Object Reference"))
  ;[0.1852 1 0] On Possess
  (bind _asbp_bat (cast `/Game/_Game/BP_Bat` PossessedPawn)
    (:`then`
      (bind _output_get (set `self.As BP Bat` _asbp_bat))
      (`Bat.SpawnBall` _output_get)
      (bind _returnvalue (`|CreateWidget` "/Game/_Game/UI/WBP_Score.WBP_Score_C" self))
      (bind _output_get_2 (set `self.Displayed Score` _returnvalue))
      (`UserWidget.AddToViewport` _output_get_2 0))
    (:`CastFailed`
      (`KismetSystemLibrary.PrintString` "Bat Cast Failed"))))

(event `InputAxis|Move`
  (params (AxisValue :type "Float (single-precision)"))
  (bind _as_bp_bat (`self.As BP Bat`))
  (bind _mouse_move_rate (`self.Mouse Move Rate`))
  ;[1 1 1] Movement
  (bind _output_get (set `self.Mouse Move Rate` (* AxisValue (`self.Mouse Sensitivity`))))
  (`/Engine/EditorBlueprintResources/StandardMacros.CompareFloat` _output_get
    (:`>`
      (`Bat.MoveRight` _as_bp_bat)
      (`Bat.SetTimelinePlayRate` _as_bp_bat _mouse_move_rate :!label _label))
    (:`==`
      (`Bat.StopMoving` _as_bp_bat))
    (:`<`
      (`Bat.MoveLeft` _as_bp_bat)
      (`/Engine/EditorBlueprintResources/StandardMacros.NegateFloat` _mouse_move_rate
        (:`  `
          (goto _label))))))

(fn `UserConstructionScript`)