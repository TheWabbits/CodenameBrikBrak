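; BP_Bat is the player's paddle in a ball-and-bat game, moving along a spline and spawning the ball.
; A timeline maps to distance along the spline: play, reverse and stop handle movement, play rate sets speed, and reset sets its time.
; Spawning a ball switches the bat to Active, where ball destruction sends a life-loss message to the PlayerState and a lives update returns it to Setup.
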(event `self.ReceiveBeginPlay`
  (`self.ResetBat`))

(event `self.SpawnBall`
  (`self.Change Player State` "NewEnumerator1")
  (bind _returnvalue (`|SpawnActorFromClass` "/Game/_Game/BP_Ball.BP_Ball_C" (`SceneComponent.K2_GetComponentToWorld` (`self.Arrow_BatSpawnPoint`)) "AlwaysSpawn" "OverrideRootScale" null null))
  (add `Actor.OnDestroyed` _returnvalue (delegate `Ball Destroyed`)))

(event `Ball Destroyed`
  (params (DestroyedActor :type "Actor Object Reference"))
  (switch `/Game/_Game/Core/PlayerState/ENUM_BatState` (`self.Bat State`)
    (:`NewEnumerator1`
      (`self.LoseLife`))))

(event `self.MoveRight`
  (bind _spline (`self.Spline`))
  (bind (_direction _bat_position_on_spline) (`Timeline|Bat Timeline` :`NewTime` 0.5 :!label _label)
    (:`Update`
      (bind (_returnvalue_location _returnvalue_rotation) (`KismetMathLibrary.BreakTransform` (`SplineComponent.GetTransformAtDistanceAlongSpline` _spline (* (`SplineComponent.GetSplineLength` _spline) _bat_position_on_spline) "World" false)))
      (`SceneComponent.K2_SetWorldTransform` (`self.BatAnchor`) (`KismetMathLibrary.MakeTransform` _returnvalue_location _returnvalue_rotation) true false))))

(event `self.StopMoving`
  (goto _label :!via `Stop`))

(event `self.MoveLeft`
  (goto _label :!via `Reverse`))

(event `self.ResetBat`
  (goto _label :!via `SetNewTime`))

(event `self.SetTimelinePlayRate`
  (params (PlayRate :type "Float (single-precision)"))
  (`TimelineComponent.SetPlayRate` (`self.Bat Timeline`) PlayRate))

(event `self.LoseLife`
  (message `I_Framework.LivesUpdate` (`GameplayStatics.GetPlayerState` 0) -1))

(event `self.UpdatePlayerLives`
  (switch `/Game/_Game/Core/PlayerState/ENUM_BatState` (`self.Bat State`)
    (:`NewEnumerator1`
      (`self.Change Player State` "NewEnumerator0"))))

(fn `Change Player State`
  (params (`New State` :type "/Game/_Game/Core/PlayerState/ENUM_BatState Enum" :default "NewEnumerator0"))
  (if (`|EnumInequality` `New State` (`self.Bat State`))
    (set `self.Bat State` `New State`)))

(fn `UserConstructionScript`)